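; Base Gameplay Ability for RetroFPS weapons, with FireWeapon left for child abilities to override.
; Activation commits, starts a gameplay event listener, fires, then ends after the remaining cooldown.
; ApplyEffect sends the hit RetroFPSCharacter as target data to the attacker's instigator via WeaponEventTag, and the listener applies WeaponEffect to it.
; Ending the ability cleans up both async tasks and calls an empty Reset hook.
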(event Custom|WaitForEvent
  ;[0 0 0] Wait for gameplay tag
  (bind (_asynctaskproxy _payload) (Ability|Tasks|WaitGameplayEvent (Variables|Default|GetWeaponEventTag) 0)
    (:then
      (Variables|Default|SetGameplayEventWaitTask _asynctaskproxy))
    (:EventReceived
      (GameplayEffects|ApplyGameplayEffectToTarget (.TargetData (Utilities|Struct|BreakGameplayEventData _payload)) (Variables|Default|GetWeaponEffect) 1 1))))

(event Custom|Fire%20Weapon
  ;[1 0.9385 0] To override
)

(event Ability|EventActivateAbility
  ;[0 0 0] Activate ability
  (Ability|CommitAbility)
  (CallFunction|WaitforEvent)
  (CallFunction|FireWeapon)
  ;[0 0 0] Ability cooldown
  (bind _asynctaskproxy (GameplayTasks|TaskWaitDelay 0 (Class|GameplayAbility|GetCooldownTimeRemaining))
    (:then
      (Variables|Default|SetFireWaitDelayTask _asynctaskproxy))
    (:OnFinish
      (Ability|EndAbility))))

(event Ability|EventOnEndAbility
  (params (bWasCancelled :type Boolean))
  (bind _gameplayeventwaittask (Variables|Default|GetGameplayEventWaitTask))
  (bind _firewaitdelaytask (Variables|Default|GetFireWaitDelayTask))
  ;[0 0 0] End ability and clean
  (Utilities|IsValid _gameplayeventwaittask
    (:Is%20Valid
      (GameplayTasks|EndTask _gameplayeventwaittask))
    (:Is%20Not%20Valid
      _))
  (Utilities|IsValid _firewaitdelaytask
    (:Is%20Valid
      (GameplayTasks|EndTask _firewaitdelaytask)
      (CallFunction|Reset))))

(fn Reset)

(fn ApplyEffect
  (params (AttackingActor :type Actor%20Object%20Reference) (TargetActor :type Actor%20Object%20Reference))
  (bind _asretro_fpscharacter (Utilities|Casting|CastToRetroFPSCharacter TargetActor))
  (Ability|SendGameplayEventtoActor (Variables|/Script/Engine.Actor|GetInstigator AttackingActor) (Variables|Default|GetWeaponEventTag) (Utilities|Struct|MakeGameplayEventData "(TagName=\"\")" 0 _asretro_fpscharacter 0 0 "()" "(GameplayTags=)" "(GameplayTags=)" 0.0 (Ability|TargetData|AbilityTargetDatafromActor _asretro_fpscharacter))))