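; Gameplay ability that gives the Outlander enemy a hitscan pistol attack against the player character.
; FireWeapon caches the owning enemy, then line-traces forward from its capsule over WeaponRange, leaving persistent debug drawing.
; A hit RetroFPSCharacter receives the ability's effect.
; When the trace returns no valid actor, a pooled object from the enemy is placed at the impact point, aligned to the normal.
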(event Ability|EventActivateAbility
  (|CallParentFunction) ; This node is disabled and will not be called.\nDrag off pins to build functionality.
)

(event Ability|EventOnEndAbility
  (params (bWasCancelled :type Boolean))
  (|CallParentFunction bWasCancelled) ; This node is disabled and will not be called.\nDrag off pins to build functionality.
)

(event EventFireWeapon
  (CallFunction|GetEnemy)
  (bind _actor (CallFunction|GetLineTrace))
  (bind _asretro_fpscharacter (Utilities|Casting|CastToRetroFPSCharacter _actor))
  (CallFunction|ApplyEffect (Variables|Default|GetOutlanderEnemy) _asretro_fpscharacter))

(fn GetLineTrace
  (bind _outlanderenemy (Variables|Default|GetOutlanderEnemy))
  (bind _capsulecomponent (Variables|/Script/Engine.Character|GetCapsuleComponent _outlanderenemy))
  (bind _returnvalue (Transformation|GetWorldLocation _capsulecomponent))
  (bind _outhit (Collision|LineTraceByChannel _returnvalue (+ _returnvalue (* (Math|Vector|GetForwardVector (Transformation|GetWorldRotation _capsulecomponent)) (Variables|Default|GetWeaponRange))) "TraceTypeQuery1" false 0 "Persistent"))
  (Utilities|IsValid (.HitActor (Collision|BreakHitResult _outhit))
    (:Is%20Valid
      (return (.HitActor (Collision|BreakHitResult _outhit))))
    (:Is%20Not%20Valid
      (bind _returnvalue_2 (Class|ActorObjectPool|SpawnPooledObject (Variables|/Game/RetroFPS/BPS/Enemies/BP_OutlanderEnemy.BP_OutlanderEnemy_C|GetActorObjectPool (Variables|Default|GetOutlanderEnemy))))
      (Transformation|SetActorLocation _returnvalue_2 (.ImpactPoint (Collision|BreakHitResult _outhit)) false false)
      (Transformation|SetActorRotation _returnvalue_2 (Math|Conversions|RotationFromXVector (.ImpactNormal (Collision|BreakHitResult _outhit)))))))

(fn GetEnemy
  (Utilities|IsValid (Variables|Default|GetOutlanderEnemy)
    (:Is%20Valid
      _)
    (:Is%20Not%20Valid
      (bind _asbp_outlander_enemy (Utilities|Casting|CastToBP_OutlanderEnemy (.owneractor (Ability|GetActorInfo))))
      (Variables|Default|SetOutlanderEnemy _asbp_outlander_enemy)))
  (return))