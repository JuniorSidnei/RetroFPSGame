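; Health or shield pickup for the RetroFPS game, shown as a Paper2D flipbook.
; The construction script uses the Type setting to pick the flipbook and the matching pickup gameplay tag.
; Two check functions read a GAS attribute and add or remove a Full tag on the pickup's own tag container, comparing against a hard-coded maximum.
; The event graph is empty, and nothing in this Blueprint calls those checks.
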(event EventBeginPlay)

(event Collision|EventActorBeginOverlap
  (params (OtherActor :type Actor%20Object%20Reference)))

(event EventTick
  (params (DeltaSeconds :type Float%20%28single-precision%29))
  (|CallParentFunction DeltaSeconds) ; This node is disabled and will not be called.\nDrag off pins to build functionality.
)

(fn ConstructionScript
  (|CallParentFunction)
  (CallFunction|SetFlipBook))

(fn SetFlipBook
  (bind _item (Variables|Default|GetItem))
  (switch Utilities|FlowControl|Switch|SwitchonENUM_PickUpType (Variables|Default|GetType)
    (:NewEnumerator0
      (Sprite|SetFlipbook _item "/Game/RetroFPS/Flipbooks/PickUps/FP_HealthPickUp.FP_HealthPickUp")
      (Variables|Default|SetPickupTag "(GameplayTags=((TagName=\"PickUp.Health\")))"))
    (:NewEnumerator1
      (Sprite|SetFlipbook _item "/Game/RetroFPS/Flipbooks/PickUps/FB_ShieldPickUp.FB_ShieldPickUp")
      (Variables|Default|SetPickupTag "(GameplayTags=((TagName=\"PickUp.Shield\")))"))))

(fn FullHealthCheck
  (params (AbilitySystem :type Ability%20System%20Component%20Object%20Reference))
  (bind _pickuptag (Variables|Default|GetPickupTag))
  (if (== (.ReturnValue (Ability|Attribute|GetFloatAttributefromAbilitySystemComponent AbilitySystem "(AttributeName=\"Health\",Attribute=/Script/RetroFPS.RetroFPSAttributeSet:Health,AttributeOwner=\"/Script/CoreUObject.Class'/Script/RetroFPS.RetroFPSAttributeSet'\")")) 1e+02)
    (GameplayTags|AddGameplayTag _pickuptag "(TagName=\"Player.Health.Full\")" :!class /Script/GameplayTags.BlueprintGameplayTagLibrary)
    (else
      (GameplayTags|RemoveGameplayTag _pickuptag "(TagName=\"Player.Health.Full\")" :!class /Script/GameplayTags.BlueprintGameplayTagLibrary))))

(fn FullShieldCheck
  (params (AbilitySystem :type Ability%20System%20Component%20Object%20Reference))
  (bind _pickuptag (Variables|Default|GetPickupTag))
  (if (== (.ReturnValue (Ability|Attribute|GetFloatAttributefromAbilitySystemComponent AbilitySystem "(AttributeName=\"Armor\",Attribute=/Script/RetroFPS.RetroFPSAttributeSet:Armor,AttributeOwner=\"/Script/CoreUObject.Class'/Script/RetroFPS.RetroFPSAttributeSet'\")")) 1e+02)
    (GameplayTags|AddGameplayTag _pickuptag "(TagName=\"Player.Shield.Full\")" :!class /Script/GameplayTags.BlueprintGameplayTagLibrary)
    (else
      (GameplayTags|RemoveGameplayTag _pickuptag "(TagName=\"Player.Shield.Full\")" :!class /Script/GameplayTags.BlueprintGameplayTagLibrary))))