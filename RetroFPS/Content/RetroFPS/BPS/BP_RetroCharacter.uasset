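; BP_RetroCharacter is a RetroFPS character Blueprint that uses the Gameplay Ability System and provides health debug output.
; BeginPlay waits a tick, then prints the base value of an AbilitySystemComponent attribute, labeled as current health.
; TakeDamage receives cue data, reports a damage event at the cue location with its instigator, likely for AI perception, then prints health again.
; Overlap, Tick and construction logic are empty.
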(event Custom|Take%20Damage
  (params (CueData :type Gameplay%20Cue%20Parameters%20Structure))
  (bind (_normalizedmagnitude _rawmagnitude _effectcontext _matchedtagname _originaltag _aggregatedsourcetags _aggregatedtargettags _location _normal _instigator) (Ability|GameplayCue|BreakGameplayCueParameters CueData))
  (Class|AISenseDamage|ReportDamageEvent self _instigator 0.0 _location "0, 0, 0" "None")
  (Development|PrintString (Utilities|String|Append (Utilities|GetDisplayName self) "'s current health is at: " (Utilities|String|ToString(Float) (.ReturnValue (Class|AbilitySystemBlueprintLibrary|GetFloatAttributeBasefromAbilitySystemComponent (Variables|Default|GetAbilitySystemComponent) "(AttributeName=\"Health\",Attribute=/Script/RetroFPS.RetroFPSAttributeSet:Health,AttributeOwner=\"/Script/CoreUObject.Class'/Script/RetroFPS.RetroFPSAttributeSet'\")")))) true true "(R=0.000000,G=0.660000,B=1.000000,A=1.000000)" 1e+01))

(event EventBeginPlay
  (Utilities|FlowControl|Delay 0.0)
  (Development|PrintString (Utilities|String|Append (Utilities|GetDisplayName self) "'s current health is at:" (Utilities|String|ToString(Float) (.ReturnValue (Class|AbilitySystemBlueprintLibrary|GetFloatAttributeBasefromAbilitySystemComponent (Variables|Default|GetAbilitySystemComponent) "(AttributeName=\"Health\",Attribute=/Script/RetroFPS.RetroFPSAttributeSet:Health,AttributeOwner=\"/Script/CoreUObject.Class'/Script/RetroFPS.RetroFPSAttributeSet'\")")))) true true "(R=0.000000,G=0.660000,B=1.000000,A=1.000000)" 1e+01))

(event Collision|EventActorBeginOverlap
  (params (OtherActor :type Actor%20Object%20Reference)))

(event EventTick
  (params (DeltaSeconds :type Float%20%28single-precision%29)))

(fn ConstructionScript)