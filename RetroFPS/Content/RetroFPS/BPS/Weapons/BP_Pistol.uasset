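; BP_Pistol is the pistol weapon Blueprint for a retro FPS, handling the flipbook sprite visuals and muzzle flash.
; Initialize shows the weapon flipbook in its idle animation.
; ShootPistol triggers a brief point light flash and plays the fire flipbook, using a delay matched to the flipbook's length before returning to idle.
; The graph contains only presentation logic, with no hit detection, damage or ammo handling.
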(event Custom|Shoot%20Pistol
  (bind _weaponflipbook (Variables|Default|GetWeaponFlipbook))
  ;[0 0 0] Fire Animation
  (CallFunction|LightFlash)
  (Sprite|SetFlipbook _weaponflipbook (Variables|Default|GetFire))
  (Utilities|FlowControl|Delay (Class|PaperFlipbookComponent|GetFlipbookLength _weaponflipbook))
  (Sprite|SetFlipbook (Variables|Default|GetWeaponFlipbook) (Variables|Default|GetIdle)))

(event Custom|Light%20Flash
  (bind _pointlight (Variables|Default|GetPointLight))
  ;[0 0 0] Light Flash
  (Development|SetHiddeninGame _pointlight false false)
  (Utilities|FlowControl|Delay 0.2)
  (Development|SetHiddeninGame _pointlight true false))

(event EventInitialize
  ;[0 0 0] Equip Weapon
  (Sprite|SetFlipbook (Variables|Default|GetWeaponFlipbook) (Variables|Default|GetIdle))
  (Development|SetHiddeninGame (Variables|Default|GetWeaponFlipbook) false false))

(fn ConstructionScript
  (|CallParentFunction))