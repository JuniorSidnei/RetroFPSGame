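; Rocket launcher weapon for the retro FPS, drawn as a flipbook sprite, that fires BP_RocketProjectile actors.
; Initialize shows the sprite in its idle animation and caches the BP_FPSPlayer pawn.
; FireWeapon briefly flashes a point light, refreshes the player's UI and spawns a rocket at the Spawn component's transform.
; It then plays the fire flipbook, using a delay of that flipbook's length before returning to idle.
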(event Custom|Fire%20Weapon
  (bind _weaponflipbook (Variables|Default|GetWeaponFlipbook))
  ;[0 0 0] Fire Animation
  (CallFunction|LightFlash)
  (Default|UpdateUI (Variables|Default|GetPlayer))
  (Game|SpawnActorfromClass "/Game/RetroFPS/BPS/Projectiles/BP_RocketProjectile.BP_RocketProjectile_C" (Transformation|GetWorldTransform (Variables|Default|GetSpawn)) "Undefined" "MultiplyWithRoot" 0 0)
  (Sprite|SetFlipbook _weaponflipbook (Variables|Default|GetFire))
  (Utilities|FlowControl|Delay (Class|PaperFlipbookComponent|GetFlipbookLength _weaponflipbook))
  (Sprite|SetFlipbook (Variables|Default|GetWeaponFlipbook) (Variables|Default|GetIdle)))

(event Custom|Light%20Flash
  (bind _pointlight (Variables|Default|GetPointLight))
  ;[0 0 0] Light Flash
  (Development|SetHiddeninGame _pointlight false false)
  (Utilities|FlowControl|Delay 0.2)
  (Development|SetHiddeninGame _pointlight true false))

(event EventInitialize
  ;[0 0 0] Equip Weapon
  (Sprite|SetFlipbook (Variables|Default|GetWeaponFlipbook) (Variables|Default|GetIdle))
  (Development|SetHiddeninGame (Variables|Default|GetWeaponFlipbook) false false)
  (bind _asbp_fpsplayer (Utilities|Casting|CastToBP_FPSPlayer (Game|Player|GetPlayerPawn 0)))
  (Variables|Default|SetPlayer _asbp_fpsplayer))

(fn ConstructionScript
  (|CallParentFunction))