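; Base weapon Blueprint for a retro FPS, displaying the player's weapon as a flipbook isolated in a SceneCapture2D.
; BeginPlay restricts the capture to the flipbook and caches its rest position, while Initialize sets and unhides the flipbook.
; Show plays the draw sequence and immediately sets FinishedDraw, which gates WeaponBobbing.
; Bobbing plays a sequence while moving, otherwise stops it and interpolates the flipbook back toward rest.
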(event Custom|WeaponBobbing
  (params (isMoving :type Boolean) (deltaTime :type Float%20%28double-precision%29))
  (bind _weaponbob (Variables|Default|GetWeaponBob))
  (bind _weaponflipbook (Variables|Default|GetWeaponFlipbook))
  (bind _sequenceplayer (Variables|/Script/ActorSequence.ActorSequenceComponent|GetSequencePlayer _weaponbob))
  ;[0 0 0] Weapon start/stop bobbing
  (if (Variables|Default|GetfinishedDraw)
    (if isMoving
      (Sequencer|Player|Play _sequenceplayer :!class /Script/MovieScene.MovieSceneSequencePlayer)
      (else
        (Sequencer|Player|Stop _sequenceplayer :!class /Script/MovieScene.MovieSceneSequencePlayer)
        (Transformation|SetRelativeLocation _weaponflipbook (Math|Interpolation|VInterpTo (Variables|/Script/Engine.SceneComponent|GetRelativeLocation _weaponflipbook) (Variables|Default|GetweaponPosition) deltaTime 0.2) false false)))))

(event EventBeginPlay
  (Rendering|SceneCapture|ShowOnlyComponent (Variables|Default|GetSceneCaptureComponent2D) (Variables|Default|GetWeaponFlipbook))
  (Variables|Default|SetweaponPosition (Variables|/Script/Engine.SceneComponent|GetRelativeLocation (Variables|Default|GetWeaponFlipbook))))

(event EventInitialize
  (bind _weaponflipbook (Variables|Default|GetWeaponFlipbook))
  (Sprite|SetFlipbook _weaponflipbook)
  (Development|SetHiddeninGame _weaponflipbook false false))

(event EventShow
  ;[0 0 0] Draw weapon
  (Sequencer|Player|Play (Variables|/Script/ActorSequence.ActorSequenceComponent|GetSequencePlayer (Variables|Default|GetWeaponDraw)) :!class /Script/MovieScene.MovieSceneSequencePlayer)
  (Variables|Default|SetfinishedDraw true))

(fn ConstructionScript)