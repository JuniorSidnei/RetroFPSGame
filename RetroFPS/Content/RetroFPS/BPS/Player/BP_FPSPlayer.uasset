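; Player character for the retro FPS, handling movement, mouse look, weapon bobbing, and a HUD showing health, shield and ammo with damage and pickup flashes.
; Weapon pickups resolve through DT_Weapons, adding and equipping new weapons or granting ammo for owned ones, with input cycling the inventory.
; The equipped weapon is a swapped Child Actor.
; Firing, damage and ammo gain activate Gameplay Ability System abilities by tag, while the HUD reads attributes.
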(event Custom|Equip%20%20Weapon
  (params (Weapon :type ST%20Weapon%20Data%20Structure))
  ;[0 0 0] Equip Weapon
  (bind _output_get (Variables|Player|SetcurrentWeapon Weapon))
  (bind _weaponactor (CallFunction|InitializeWeapon (.Weapon (Utilities|Struct|BreakST_WeaponData _output_get))))
  (Class|BPIPlayerWeapon|Show(Message) _weaponactor)
  (Default|WeaponSwitchedEvent (Variables|Default|GetHUD) (.WeaponNType (Utilities|Struct|BreakST_WeaponData (Variables|Player|GetcurrentWeapon))))
  (CallFunction|UpdateUI)
  (Variables|Default|SetWeaponFire%20Tag%20Container (.WeaponTag (Utilities|Struct|BreakST_WeaponData (Variables|Player|GetcurrentWeapon)))))

(event Custom|Item%20Pickup
  ;[0 0 0] Pickup item
  (CallFunction|UpdateUI)
  (bind _flash_intensity (Timeline|Timeline PlayFromStart)
    (:Update
      (Default|SetFlashColor (Variables|Default|GetHUD) "(R=0.000000,G=0.239107,B=1.000000,A=1.000000)" _flash_intensity))))

(event Custom|PickupWeapon
  (params (Weapon :type ENUM_Weapons%20Enum :default "NewEnumerator0"))
  ;[0 0 0] Weapon pickup
  (bind (_weapondata _weaponfound) (CallFunction|GetWeaponfromDataTable Weapon))
  (if _weaponfound
    (bind _output_get (Variables|Default|SetWeaponToPickup _weapondata))
    (if (CallFunction|HasWeapon (.WeaponNType (Utilities|Struct|BreakST_WeaponData _output_get)))
      (CallFunction|AddAmmo (.AmmoType (Utilities|Struct|BreakST_WeaponData _output_get)))
      (else
        (CallFunction|AddWeapon)))))

(event Custom|Add%20ammo
  (params (AmmoType :type ENUM_AmmoType%20Enum :default "NewEnumerator2"))
  ;[0 0 0] Add ammo
  (switch Utilities|FlowControl|Switch|SwitchonENUM_AmmoType AmmoType
    (:NewEnumerator0
      (CallFunction|AddPistolBullets))
    (:NewEnumerator1
      (CallFunction|AddRocketLauncherBullets))))

(event Custom|Add%20weapon
  (bind _weapontopickup (Variables|Default|GetWeaponToPickup))
  ;[0 0 0] Add weapon
  (Utilities|Array|Add (Variables|Player|GetPlayerWeapons) _weapontopickup)
  (CallFunction|EquipWeapon _weapontopickup)
  (CallFunction|AddAmmo (.AmmoType (Utilities|Struct|BreakST_WeaponData _weapontopickup)))
  (Variables|Player|SetcurrentWeaponIndex (+ (Variables|Player|GetcurrentWeaponIndex) 1)))

(event EventBeginPlay
  ;[0 0 0] Initialization
  (|CallParentFunction)
  (bind _returnvalue (UserInterface|CreateWidget "/Game/RetroFPS/BPS/Widgets/WBP_HUD.WBP_HUD_C"))
  (bind _output_get (Variables|Default|SetHUD _returnvalue))
  (UserInterface|Viewport|AddtoViewport _output_get 0)
  (Utilities|FlowControl|Delay 0.0)
  (CallFunction|InitializeWeapon "/Game/RetroFPS/BPS/Player/BP_WeaponBase.BP_WeaponBase_C")
  (CallFunction|UpdateUI)
  (Default|WeaponSwitchedEvent (Variables|Default|GetHUD) "NewEnumerator0"))

(event EventTick
  (params (DeltaSeconds :type Float%20%28single-precision%29))
  ;[0 0 0] Weapon bobbing
  (bind _asbp_weapon_base (Utilities|Casting|CastToBP_WeaponBase (Variables|/Script/Engine.ChildActorComponent|GetChildActor (Variables|Default|GetWeapon))))
  (Default|WeaponBobbing _asbp_weapon_base (> (Math|Vector|VectorLength (Variables|/Script/Engine.MovementComponent|GetVelocity (Variables|Character|GetCharacterMovement))) 0.0) DeltaSeconds))

(event EventTakeDamage
  (params (CueData :type Gameplay%20Cue%20Parameters%20Structure))
  ;[0 0 0] Take damage
  (|CallParentFunction CueData)
  (CallFunction|UpdateUI)
  (bind _flash_intensity (Timeline|DamageFash PlayFromStart)
    (:Update
      (Default|SetFlashColor (Variables|Default|GetHUD) "(R=1.000000,G=0.000000,B=0.000000,A=1.000000)" _flash_intensity))))

(event EventDamage
  (params (DamageTag :type Gameplay%20Tag%20Container%20Structure))
  (Abilities|TryActivateAbilitiesbyTag (Variables|Default|GetAbilitySystemComponent) DamageTag true))

(event Input|ActionEvents|InputActionFireWeapon
  (params (Key :type Key%20Structure :default "None"))
  ;[0 0 0] Input fire
  (:Pressed
    (Abilities|TryActivateAbilitiesbyTag (Variables|Default|GetAbilitySystemComponent) (Variables|Default|GetWeaponFire%20Tag%20Container) false)))

(event Input|ActionEvents|InputActionChangeWeapon
  (params (Key :type Key%20Structure :default "None"))
  ;[0 0 0] Change next weapon
  (:Pressed
    (if (> (Utilities|Array|Length (Variables|Player|GetPlayerWeapons)) 0)
      (bind _output_get (Variables|Player|SetcurrentWeaponIndex (+ (Variables|Player|GetcurrentWeaponIndex) 1)))
      (if (>= _output_get (Utilities|Array|Length (Variables|Player|GetPlayerWeapons)))
        (bind _output_get_2 (Variables|Player|SetcurrentWeaponIndex 0))
        (CallFunction|EquipWeapon (Utilities|Array|Get(acopy) (Variables|Player|GetPlayerWeapons) _output_get_2))
        (else
          (CallFunction|EquipWeapon (Utilities|Array|Get(acopy) (Variables|Player|GetPlayerWeapons) (Variables|Player|GetcurrentWeaponIndex))))))))

(event Input|AxisEvents|InputAxisForward/BackwardMovement
  (params (AxisValue :type Float%20%28single-precision%29))
  ;[0 0 0] Movement
  (Pawn|Input|AddMovementInput (Math|Vector|GetForwardVector (Math|Rotator|MakeRotator 0.0 0.0 (.yaw (Pawn|GetControlRotation :!class /Script/Engine.Pawn)))) AxisValue false))

(event Input|AxisEvents|InputAxisRight/LeftMovement
  (params (AxisValue :type Float%20%28single-precision%29))
  ;[0 0 0] Movement
  (Pawn|Input|AddMovementInput (Math|Vector|GetRightVector (Math|Rotator|MakeRotator 0.0 0.0 (.yaw (Pawn|GetControlRotation :!class /Script/Engine.Pawn)))) AxisValue false))

(event Input|AxisEvents|InputAxisMouseLookHorizontal
  (params (AxisValue :type Float%20%28single-precision%29))
  ;[0 0 0] Mouse look
  (Pawn|Input|AddControllerYawInput AxisValue))

(event Input|AxisEvents|InputAxisMouseLookVertical
  (params (AxisValue :type Float%20%28single-precision%29))
  ;[0 0 0] Mouse look
  (Pawn|Input|AddControllerPitchInput AxisValue))

(fn ConstructionScript)

(fn UpdateUI
  (bind _abilitysystemcomponent (Variables|Default|GetAbilitySystemComponent))
  (bind _hud (Variables|Default|GetHUD))
  (bind _hud_2 (Variables|Default|GetHUD))
  (bind _ammo_txt (Variables|/Game/RetroFPS/BPS/Widgets/WBP_HUD.WBP_HUD_C|Getammo_txt _hud))
  (Rendering|Components|TextRender|SetText (Variables|/Game/RetroFPS/BPS/Widgets/WBP_HUD.WBP_HUD_C|Gethealth_txt _hud_2) (Utilities|Text|ToText(Float) (.ReturnValue (Ability|Attribute|GetFloatAttributefromAbilitySystemComponent _abilitysystemcomponent "(AttributeName=\"Health\",Attribute=/Script/RetroFPS.RetroFPSAttributeSet:Health,AttributeOwner=\"/Script/CoreUObject.Class'/Script/RetroFPS.RetroFPSAttributeSet'\")")) "HalfToEven"))
  (Rendering|Components|TextRender|SetText (Variables|/Game/RetroFPS/BPS/Widgets/WBP_HUD.WBP_HUD_C|Getshield_txt _hud_2) (Utilities|Text|ToText(Float) (.ReturnValue (Ability|Attribute|GetFloatAttributefromAbilitySystemComponent _abilitysystemcomponent "(AttributeName=\"Armor\",Attribute=/Script/RetroFPS.RetroFPSAttributeSet:Armor,AttributeOwner=\"/Script/CoreUObject.Class'/Script/RetroFPS.RetroFPSAttributeSet'\")")) "HalfToEven"))
  (switch Utilities|FlowControl|Switch|SwitchonENUM_AmmoType (.AmmoType (Utilities|Struct|BreakST_WeaponData (Variables|Player|GetcurrentWeapon)))
    (:NewEnumerator0
      (Variables|/Script/UMG.TextBlock|SetText _ammo_txt (Utilities|Text|ToText(Float) (.ReturnValue (Ability|Attribute|GetFloatAttributefromAbilitySystemComponent (Variables|Default|GetAbilitySystemComponent) "(AttributeName=\"PistolAmmo\",Attribute=/Script/RetroFPS.RetroFPSAttributeSet:PistolAmmo,AttributeOwner=\"/Script/CoreUObject.Class'/Script/RetroFPS.RetroFPSAttributeSet'\")")) "HalfToEven")))
    (:NewEnumerator1
      (Variables|/Script/UMG.TextBlock|SetText _ammo_txt (Utilities|Text|ToText(Float) (.ReturnValue (Ability|Attribute|GetFloatAttributefromAbilitySystemComponent (Variables|Default|GetAbilitySystemComponent) "(AttributeName=\"RocketAmmo\",Attribute=/Script/RetroFPS.RetroFPSAttributeSet:RocketAmmo,AttributeOwner=\"/Script/CoreUObject.Class'/Script/RetroFPS.RetroFPSAttributeSet'\")")) "HalfToEven")))))

(fn HasWeapon
  (params (Weapon :type ENUM_Weapons%20Enum :default "NewEnumerator0"))
  (bind _array_element (Utilities|Array|ForEachLoopwithBreak (Variables|Player|GetPlayerWeapons) :!label _label)
    (:LoopBody
      (if (Utilities|Enum|Equal(Enum) (.WeaponNType (Utilities|Struct|BreakST_WeaponData _array_element)) Weapon)
        (LocalVariables|SetWeaponFound true)
        (goto _label Break)))
    (:Completed
      (return (LocalVariables|GetWeaponFound)))))

(fn GetWeaponfromDataTable
  (params (Weapon :type ENUM_Weapons%20Enum :default "NewEnumerator0"))
  (bind _outrownames (DataTable|GetDataTableRowNames "/Game/RetroFPS/BPS/DataBases/DT_Weapons.DT_Weapons"))
  (bind _array_element (Utilities|Array|ForEachLoopwithBreak _outrownames :!label _label)
    (:LoopBody
      (bind _returnvalue (Utilities|GetDataTableRow "/Game/RetroFPS/BPS/DataBases/DT_Weapons.DT_Weapons" _array_element)
        (:then
          (if (Utilities|Enum|Equal(Enum) Weapon (.WeaponNType (Utilities|Struct|BreakST_WeaponData _returnvalue)))
            (LocalVariables|SetWeaponToEquip _returnvalue)
            (LocalVariables|SetWeaponExists true)
            (goto _label Break)))))
    (:Completed
      (return (LocalVariables|GetWeaponToEquip) (LocalVariables|GetWeaponExists)))))

(fn AddPistolBullets
  (Variables|Default|SetAmmoGainTagContainer "(GameplayTags=((TagName=\"Pickup.Ammo.PistolBullets\")))")
  (if (not (>= (.ReturnValue (Ability|Attribute|GetFloatAttributefromAbilitySystemComponent (Variables|Default|GetAbilitySystemComponent) "(AttributeName=\"PistolAmmo\",Attribute=/Script/RetroFPS.RetroFPSAttributeSet:PistolAmmo,AttributeOwner=\"/Script/CoreUObject.Class'/Script/RetroFPS.RetroFPSAttributeSet'\")")) (Variables|Default|GetmaxPistolAmmo)))
    (Abilities|TryActivateAbilitiesbyTag (Variables|Default|GetAbilitySystemComponent) (Variables|Default|GetAmmoGainTagContainer) false)
    (CallFunction|ItemPickup)))

(fn InitializeWeapon
  (params (InClass :type BP%20Weapon%20Base%20Class%20Reference))
  (bind _weapon (Variables|Default|GetWeapon))
  (bind _childactor (Variables|/Script/Engine.ChildActorComponent|GetChildActor _weapon))
  (ChildActorComponent|SetChildActorClass _weapon InClass)
  (if (Utilities|DoesObjectImplementInterface _childactor "/Game/RetroFPS/BPS/Interfaces/BP_IPlayerWeapon.BP_IPlayerWeapon_C")
    (Class|BPIPlayerWeapon|Initialize(Message) _childactor))
  (return _childactor))

(fn AddRocketLauncherBullets
  (Variables|Default|SetAmmoGainTagContainer "(GameplayTags=((TagName=\"Pickup.Ammo.RocketLauncherBullets\")))")
  (if (not (>= (.ReturnValue (Ability|Attribute|GetFloatAttributefromAbilitySystemComponent (Variables|Default|GetAbilitySystemComponent) "(AttributeName=\"RocketAmmo\",Attribute=/Script/RetroFPS.RetroFPSAttributeSet:RocketAmmo,AttributeOwner=\"/Script/CoreUObject.Class'/Script/RetroFPS.RetroFPSAttributeSet'\")")) (Variables|Default|GetmaxRocketsAmmo)))
    (Abilities|TryActivateAbilitiesbyTag (Variables|Default|GetAbilitySystemComponent) (Variables|Default|GetAmmoGainTagContainer) false)
    (CallFunction|ItemPickup)))