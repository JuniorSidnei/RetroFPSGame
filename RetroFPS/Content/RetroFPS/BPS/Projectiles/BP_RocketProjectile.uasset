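; BP_RocketProjectile is a rocket projectile for a retro FPS, drawn as a Paper2D sprite that damages what it overlaps.
; Each Tick it billboards the sprite toward the player camera on yaw only, with a -90 degree offset and zero pitch and roll.
; When the Collider begins overlapping an actor that implements BP_IDamagable, it sends that actor a DamageMessage.
; The graph does not handle movement or destroy the rocket on impact.
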(event OnComponentBeginOverlap(collider)
  (params (OverlappedComponent :type Primitive%20Component%20Object%20Reference) (OtherActor :type Actor%20Object%20Reference) (OtherComp :type Primitive%20Component%20Object%20Reference) (OtherBodyIndex :type Integer) (bFromSweep :type Boolean) (SweepResult :type Hit%20Result%20Structure%20%28by%20ref%29))
  (if (Utilities|DoesObjectImplementInterface OtherActor "/Game/RetroFPS/BPS/Interfaces/BP_IDamagable.BP_IDamagable_C")
    (Class|BPIDamagable|Damage(Message) OtherActor)))

(event EventTick
  (params (DeltaSeconds :type Float%20%28single-precision%29))
  (Transformation|SetWorldRotation (Variables|Default|GetPaperSprite) (Math|Rotator|MakeRotator 0.0 0.0 (- (.yaw (Math|Rotator|FindLookatRotation (Transformation|GetWorldLocation (Variables|Default|GetPaperSprite)) (Camera|GetCameraLocation (Game|GetPlayerCameraManager 0)))) 9e+01)) false false))

(fn ConstructionScript)