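; BP_OutlanderEnemy is the Outlander enemy Blueprint for a retro FPS, adding a ranged attack to its parent class.
; RangedAttack activates Gameplay Ability System abilities by tag, then briefly unhides a point light as a flash before hiding it after a short delay.
; The construction script only calls the parent, and BeginPlay, overlap and Tick are disabled stubs.
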(event EventBeginPlay
  (|CallParentFunction) ; This node is disabled and will not be called.\nDrag off pins to build functionality.
)

(event Collision|EventActorBeginOverlap
  (params (OtherActor :type Actor%20Object%20Reference))
  (|CallParentFunction OtherActor) ; This node is disabled and will not be called.\nDrag off pins to build functionality.
)

(event EventTick
  (params (DeltaSeconds :type Float%20%28single-precision%29))
  (|CallParentFunction DeltaSeconds) ; This node is disabled and will not be called.\nDrag off pins to build functionality.
)

(event EventRangedAttack
  (bind _pointlight (Variables|Default|GetPointLight))
  (Abilities|TryActivateAbilitiesbyTag (Variables|Default|GetAbilitySystemComponent) (Variables|Default|GetGameplay%20Tag%20Container) false)
  (Development|SetHiddeninGame _pointlight false false)
  (Utilities|FlowControl|Delay 0.2)
  (Development|SetHiddeninGame _pointlight true false))

(fn ConstructionScript
  (|CallParentFunction))